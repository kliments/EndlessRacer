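; BP_Floor5 is a self-recycling track segment for an endless-runner style vehicle game.
; Its construction script scatters coin child actors at random points inside two box areas, and GetAttachTransform exposes the AttachPoint world transform.
; A vehicle entering EndTrigger makes the game mode call AddFloors, and any end overlap there destroys the segment after a short delay.
; Any overlap with EndGame quits the game outright.
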(event `self.EndTrigger.OnComponentBeginOverlap`
  (params (OverlappedComponent :type "PrimitiveComponent Object Reference") (OtherActor :type "Actor Object Reference") (OtherComp :type "PrimitiveComponent Object Reference") (OtherBodyIndex :type Integer) (bFromSweep :type Boolean) (SweepResult :type "HitResult Structure (by ref)"))
  (cast `/Game/VehicleAdvBP/Blueprints/Vehicle` OtherActor)
  (bind _asvehicle_adv_game_mode (cast `/Game/VehicleAdvBP/Blueprints/VehicleAdvGameMode` (`GameplayStatics.GetGameMode`)))
  (`/Game/VehicleAdvBP/Blueprints/VehicleAdvGameMode.AddFloors` _asvehicle_adv_game_mode))

(event `self.EndTrigger.OnComponentEndOverlap`
  (params (OverlappedComponent :type "PrimitiveComponent Object Reference") (OtherActor :type "Actor Object Reference") (OtherComp :type "PrimitiveComponent Object Reference") (OtherBodyIndex :type Integer))
  (`KismetSystemLibrary.Delay` 2.0)
  (`self.K2_DestroyActor`))

(event `self.EndGame.OnComponentBeginOverlap`
  (params (OverlappedComponent :type "PrimitiveComponent Object Reference") (OtherActor :type "Actor Object Reference") (OtherComp :type "PrimitiveComponent Object Reference") (OtherBodyIndex :type Integer) (bFromSweep :type Boolean) (SweepResult :type "HitResult Structure (by ref)"))
  (`KismetSystemLibrary.QuitGame` null "Quit"))

(fn `GetAttachTransform`
  (returns (AttachTransform :type "Transform Structure"))
  (return (`SceneComponent.K2_GetComponentToWorld` (`self.AttachPoint`))))

(fn `SpawnCoins`
  (bind _coinarea1 (`self.CoinArea1`))
  (bind _coinarea2 (`self.CoinArea2`))
  (`AddComponent|NODE_AddChildActorComponent-0` :`RelativeTransform` (`KismetMathLibrary.Conv_VectorToTransform` (`KismetMathLibrary.RandomPointInBoundingBox` (`SceneComponent.RelativeLocation` _coinarea1) (`BoxComponent.BoxExtent` _coinarea1))))
  (`AddComponent|NODE_AddChildActorComponent-1` :`RelativeTransform` (`KismetMathLibrary.Conv_VectorToTransform` (`KismetMathLibrary.RandomPointInBoundingBox` (`SceneComponent.RelativeLocation` _coinarea2) (`BoxComponent.BoxExtent` _coinarea2)))))

(fn `UserConstructionScript`
  (for _ (range 6)
    (`self.SpawnCoins`)))