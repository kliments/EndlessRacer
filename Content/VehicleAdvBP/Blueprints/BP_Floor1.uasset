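; BP_Floor1 is a floor segment actor that appears to support endlessly extended track for the vehicle game.
; When a VehicleBlueprint overlaps EndTrigger, it calls AddFloors on the VehicleAdvGameMode.
; When any overlap with EndTrigger ends, the segment destroys itself after a two-second delay, without checking which actor left.
; GetAttachTransform exposes the AttachPoint world transform, presumably for placing the next segment.
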(event `self.EndTrigger.OnComponentBeginOverlap`
  (params (OverlappedComponent :type "PrimitiveComponent Object Reference") (OtherActor :type "Actor Object Reference") (OtherComp :type "PrimitiveComponent Object Reference") (OtherBodyIndex :type Integer) (bFromSweep :type Boolean) (SweepResult :type "HitResult Structure (by ref)"))
  (cast `/Game/VehicleAdvBP/Blueprints/VehicleBlueprint` OtherActor)
  (bind _asvehicle_adv_game_mode (cast `/Game/VehicleAdvBP/Blueprints/VehicleAdvGameMode` (`GameplayStatics.GetGameMode`)))
  (`/Game/VehicleAdvBP/Blueprints/VehicleAdvGameMode.AddFloors` _asvehicle_adv_game_mode))

(event `self.EndTrigger.OnComponentEndOverlap`
  (params (OverlappedComponent :type "PrimitiveComponent Object Reference") (OtherActor :type "Actor Object Reference") (OtherComp :type "PrimitiveComponent Object Reference") (OtherBodyIndex :type Integer))
  (`KismetSystemLibrary.Delay` 2.0)
  (`self.K2_DestroyActor`))

(fn `GetAttachTransform`
  (returns (AttachTransform :type "Transform Structure"))
  (return (`SceneComponent.K2_GetComponentToWorld` (`self.AttachPoint`))))

(fn `UserConstructionScript`)